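; Spectator pawn that lets the player select and take control of a BaseUnit by looking at it and pressing SelectUnit.
; While player-controlled, Tick traces 500 units forward from the collision component for Pawn objects and prints the hit actor's name.
; With SelectUnit held on a BaseUnit, it disables its input and blends the camera to that unit.
; After a short delay, the player controller possesses the unit.
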(event `InputAction|SelectUnit`
  (params (Key :type "Key Structure" :default "AnyKey"))
  ;[1 1 1] Sets hasClicked true on press, false on release
  (:`Pressed`
    (set `self.hasClicked` true))
  (:`Released`
    (set `self.hasClicked` false)))

(event `self.ReceiveTick`
  (params (DeltaSeconds :type "Float (single-precision)"))
  (bind _returnvalue (`GameplayStatics.GetPlayerController` 0))
  (bind _collisioncomponent (`self.CollisionComponent`))
  (bind _returnvalue_2 (`SceneComponent.K2_GetComponentLocation` _collisioncomponent))
  ;[1 1 1] Make sure it doesn't constantly fire when not being used
  (if (`self.IsPlayerControlled`)
    (bind _outhit (`KismetSystemLibrary.LineTraceSingleForObjects` _returnvalue_2 (+ _returnvalue_2 (* (`KismetMathLibrary.GetForwardVector` (`SceneComponent.K2_GetComponentRotation` _collisioncomponent)) 500.0)) (`|MakeArray` "ObjectTypeQuery3" :!type "EObjectTypeQuery Enum")))
    (bind (_bblockinghit _binitialoverlap _time _location _impactpoint _normal _impactnormal _physmat _hitactor) (`GameplayStatics.BreakHitResult` _outhit))
    (`KismetSystemLibrary.PrintString` (`KismetSystemLibrary.GetDisplayName` _hitactor) true true (struct :`G` 0.66 :`B` 1.0 :`A` 1.0) 0.2)
    (if (and (`self.hasClicked`) (`KismetMathLibrary.ClassIsChildOf` (`GameplayStatics.GetObjectClass` _hitactor) "/Game/Blueprints/BaseUnit.BaseUnit_C"))
      ;[1 1 1] Stops weird stuff from happening
      (`self.DisableInput` _returnvalue)
      ;[1 1 1] Blend camera to move to selected unit before possessing unit
      (`PlayerController.SetViewTargetWithBlend` _returnvalue _hitactor 0.5 "VTBlend_Linear" 0.0 false)
      (`KismetSystemLibrary.Delay` 0.75)
      (bind _asbase_unit (cast `/Game/Blueprints/BaseUnit` _hitactor))
      (`Controller.Possess` _returnvalue _asbase_unit))))

(fn `UserConstructionScript`)